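; Data wrapper for a single inventory item, exposing its item record, expiration time and parent through getters.
; GetGroups fills a map of group external IDs to names, and GetIsHidden checks the attributes for a "HideIn" entry with value "Inventory".
; RefreshIcon stores a supplied icon and sets a ready flag, readable through IsIconSet, alongside the raw image URL.
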(event `/XsollaInventory/Common/Interface/BPI_IconPresenter.RefreshIcon`
  (params (Icon :type "SlateBrush Structure"))
  (set `self.Icon` Icon)
  (set `self.IsIconReady` true))

(fn `GetDescription`
  (returns (Description :type String))
  (return (`.description` (break `InventoryItem` (`self.ItemData`)))))

(fn `GetExpirationTime`
  (returns (ExpiresAt :type Integer64))
  (return (`self.ExpiresAt`)))

(fn `GetGroups`
  (returns (Groups :type "Map of String to String"))
  (locals (ItemGroups :type "Map of String to String"))
  (for _array_element (`.groups` (break `InventoryItem` (`self.ItemData`)))
    (bind (_id _external_id _name) (break `XsollaItemGroup` _array_element))
    (`BlueprintMapLibrary.Map_Add` (`local.ItemGroups`) _external_id _name))
  (return (`local.ItemGroups`)))

(fn `GetIcon`
  (returns (Icon :type "SlateBrush Structure"))
  (return (`self.Icon`)))

(fn `GetImageUrl`
  (returns (ImageUrl :type String))
  (return (`.image_url` (break `InventoryItem` (`self.ItemData`)))))

(fn `GetInstanceId`
  (returns (InstanceId :type String))
  (return (`.instance_id` (break `InventoryItem` (`self.ItemData`)))))

(fn `GetIsHidden`
  (returns (IsHidden :type Boolean))
  (locals (attributes :type "Array of XsollaItemAttribute Structure"))
  (bind _output_get (set `local.attributes` (`.attributes` (break `InventoryItem` (`self.ItemData`)))))
  (for _array_element _output_get
    (bind (_external_id _name _values) (break `XsollaItemAttribute` _array_element))
    (if (`KismetStringLibrary.EqualEqual_StrStr` _name "HideIn")
      (for _array_element_2 _values
        (if (`KismetStringLibrary.EqualEqual_StrStr` (`.value` (break `XsollaItemAttributeValue` _array_element_2)) "Inventory")
          (return true)))))
  (return false))

(fn `GetName`
  (returns (Name :type String))
  (return (`.name` (break `InventoryItem` (`self.ItemData`)))))

(fn `GetParent`
  (returns (Parent :type "/XsollaInventory/Inventory/Interface/BPI_InventoryPanel Interface"))
  (return (`self.Parent`)))

(fn `GetQuantity`
  (returns (Quantity :type Integer))
  (return (`.quantity` (break `InventoryItem` (`self.ItemData`)))))

(fn `GetSku`
  (returns (Sku :type String))
  (return (`.sku` (break `InventoryItem` (`self.ItemData`)))))

(fn `GetVirtualItemType`
  (returns (Type :type String))
  (return (`.virtual_item_type` (break `InventoryItem` (`self.ItemData`)))))

(fn `IsIconSet`
  (returns (IsIconSet :type Boolean))
  (return (`self.IsIconReady`)))