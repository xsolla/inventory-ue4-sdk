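; BP_TokenUtils is a set of helper functions that read the current player's auth token from the Xsolla Login subsystem.
; It returns the JWT, the refresh token, any named string claim, and the is_master flag.
; Expiration time comes from the stored ExpiresAt when OAuth2 is enabled, otherwise from the JWT's exp claim converted to int64.
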(fn `Get Token Expiration Time`
  (returns (ExpiresAt :type Integer64))
  (bind (_jwt _expiresat) (break `XsollaAuthToken` (`.AuthToken` (break `XsollaLoginData` (`XsollaLoginSubsystem.GetLoginData` (subsystem `XsollaLoginSubsystem`))))))
  (bind _paramvalue (`XsollaUtilsTokenParser.GetStringTokenParam` _jwt "exp"))
  (return (select `bool` (`/XsollaInventory/Common/BP_DemoUtils.Get Use OAuth 2` (`local.__WorldContext`)) :`false` (`KismetMathLibrary.Conv_IntToInt64` (`KismetStringLibrary.Conv_StringToInt` _paramvalue)) :`true` _expiresat)))

(fn `GetRefreshToken`
  (returns (RefreshToken :type String))
  (return (`.RefreshToken` (break `XsollaAuthToken` (`.AuthToken` (break `XsollaLoginData` (`XsollaLoginSubsystem.GetLoginData` (subsystem `XsollaLoginSubsystem`))))))))

(fn `GetToken`
  (returns (Token :type String))
  (return (`.JWT` (break `XsollaAuthToken` (`.AuthToken` (break `XsollaLoginData` (`XsollaLoginSubsystem.GetLoginData` (subsystem `XsollaLoginSubsystem`))))))))

(fn `GetTokenParameter`
  (params (Parameter :type String))
  (returns (value :type String))
  (bind _paramvalue (`XsollaUtilsTokenParser.GetStringTokenParam` (`.JWT` (break `XsollaAuthToken` (`.AuthToken` (break `XsollaLoginData` (`XsollaLoginSubsystem.GetLoginData` (subsystem `XsollaLoginSubsystem`)))))) Parameter))
  (return _paramvalue))

(fn `IsMasterAccount`
  (returns (ReturnValue :type Boolean))
  (bind _paramvalue (`XsollaUtilsTokenParser.GetBoolTokenParam` (`.JWT` (break `XsollaAuthToken` (`.AuthToken` (break `XsollaLoginData` (`XsollaLoginSubsystem.GetLoginData` (subsystem `XsollaLoginSubsystem`)))))) "is_master"))
  (return _paramvalue))